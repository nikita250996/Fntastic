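; BP_Button is a pressable button actor that tells its assigned Nest to create a turtle.
; Collision overlap sets it as the player's ActiveButton and shows a widget through BP_GameMode; leaving clears both.
; CreateTurtle triggers the Nest, disables the button and animates its Z with a timeline as a cooldown.
; When the timeline finishes, the button reactivates and re-shows the widget if the player still overlaps.
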(event `self.ReceiveBeginPlay`
  ;[1 1 1] Game Mode нужен для того, чтобы работать через него с виджетом
  (bind _asbp_game_mode (cast `/Game/Blueprints/GameModes/BP_GameMode` (`GameplayStatics.GetGameMode`)))
  (set `self.Game Mode` _asbp_game_mode))

(event `self.Collision.OnComponentBeginOverlap`
  (params (OverlappedComponent :type "PrimitiveComponent Object Reference") (OtherActor :type "Actor Object Reference") (OtherComp :type "PrimitiveComponent Object Reference") (OtherBodyIndex :type Integer) (bFromSweep :type Boolean) (SweepResult :type "HitResult Structure (by ref)"))
  ;[1 1 1] Если кнопка активна и игрок подошёл близко, указываем игроку, что он взаимодействует с этой кнопкой и активируем виджет
  (if (`self.Is Active`)
    (`self.Is Player` OtherActor
      (:`Player`
        (bind _asbp_player (cast `/Game/Blueprints/Characters/Player/BP_Player` OtherActor))
        (set `/Game/Blueprints/Characters/Player/BP_Player.Active Button` self _asbp_player) ; Игрок связан с этой кнопкой
        (`self.Add Widget`)))))

(event `self.Collision.OnComponentEndOverlap`
  (params (OverlappedComponent :type "PrimitiveComponent Object Reference") (OtherActor :type "Actor Object Reference") (OtherComp :type "PrimitiveComponent Object Reference") (OtherBodyIndex :type Integer))
  ;[1 1 1] Если игрок отошёл слишком далеко, он больше не может нажать на эту кнопку
  (`self.Is Player` OtherActor
    (:`Player`
      (bind _asbp_player (cast `/Game/Blueprints/Characters/Player/BP_Player` OtherActor))
      (set `/Game/Blueprints/Characters/Player/BP_Player.Active Button` null _asbp_player) ; Игрок больше не связан с этой кнопкой
      (`WidgetLayoutLibrary.RemoveAllWidgets`))))

(event `Create Turtle`
  (bind _nest (`self.Nest`))
  ;[1 1 1] Если кнопке назначено гнездо, нужно её нажать (отобразить это физически) и запретить на время «перезарядки» нажимать снова, а если за время перезарядки игрок не ушёл, нужно предложить ему снова нажать
  (if (`self.Is Active`)
    (`/Engine/EditorBlueprintResources/StandardMacros.IsValid` _nest ; Назначено ли гнездо
      (:`Is Valid`
        (`/Game/Blueprints/Actors/Nest/BP_Nest.Create Turtle` _nest)
        (set `self.Is Active` false) ; Снова нажать нельзя
        (bind (_direction _down_and_up_z) (`Timeline|Push Timeline` :!via `PlayFromStart`) ; Контролируем Z кнопки во времени
          (:`Update`
            (`self.Move Button` _down_and_up_z) ; Двигаем кнопку
          )
          (:`Finished`
            (set `self.Is Active` true) ; Снова можно нажать
            (`self.Is Player Still Overlapping` ; Близко ли игрок
              (:`Overlapping`
                (`self.Add Widget`)))))))))

(fn `Add Widget`
  (`/Game/Blueprints/GameModes/BP_GameMode.Add Widget` (`self.Game Mode`)))

(fn `Move Button`
  (params (Z :type "Float (double-precision)"))
  (bind (_start_location_x _start_location_y) (`KismetMathLibrary.BreakVector` (`self.Start Location`)))
  (`SceneComponent.K2_SetRelativeLocation` (`self.Button`) (`KismetMathLibrary.MakeVector` _start_location_x _start_location_y Z) false false))

(fn `UserConstructionScript`
  (set `self.Start Location` (`SceneComponent.RelativeLocation` (`self.Button`))) ; Начальное положение кнопки
)