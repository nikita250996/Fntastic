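; BP_Nest is a nest actor that spawns AI turtles and sends them toward a designer-set destination.
; On BeginPlay it moves its DestinationPoint component to the per-instance relative location.
; CreateTurtle, which is not called within this Blueprint, checks the turtle class, spawns it at TurtleSpawnPoint, then casts it to BP_Turtle.
; It passes the destination's world location to the turtle and starts its movement.
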(event `self.ReceiveBeginPlay`
  ;[1 1 1] Переместить точку назначения черепашки в заданную геймдизайнером для конкретного гнезда на сцене локацию
  (`self.Set Destiantion Point Location`))

(fn `Create Turtle`
  (`self.Is Turtle Class Valid` ; Задана ли определённая разновидность черепашки
    (:`Is Valid`
      (bind _returnvalue (`self.Spawn Turtle`)) ; Поместить нужную черепашку в мир
      (`self.Setup Turtle` _returnvalue) ; Задать ей параметры
    )))

(fn `Set Destiantion Point Location`
  (`SceneComponent.K2_SetRelativeLocation` (`self.Destination Point`) (`self.Destination Point Location`) false false))

(fn `Setup Turtle`
  (params (Turtle :type "Object Object Reference"))
  (bind _asbp_turtle (cast `/Game/Blueprints/Characters/Turtles/BP_Turtle` Turtle))
  (`/Game/Blueprints/Characters/Turtles/BP_Turtle.Set Destination Point Location` _asbp_turtle (`SceneComponent.K2_GetComponentLocation` (`self.Destination Point`))) ; Задать черепашке точку назначения
  (`/Game/Blueprints/Characters/Turtles/BP_Turtle.Start Moving` _asbp_turtle) ; Отправить черепашку точку назначения
)

(fn `Spawn Turtle`
  (returns (ReturnValue :type "Pawn Object Reference"))
  (bind _turtle_spawn_point (`self.Turtle Spawn Point`))
  (bind _returnvalue (`AIBlueprintHelperLibrary.SpawnAIFromClass` (`self.Turtle`) null (`SceneComponent.K2_GetComponentLocation` _turtle_spawn_point) (`SceneComponent.K2_GetComponentRotation` _turtle_spawn_point) false null))
  (return _returnvalue))

(fn `UserConstructionScript`)