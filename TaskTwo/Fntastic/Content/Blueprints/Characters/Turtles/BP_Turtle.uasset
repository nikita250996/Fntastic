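; BP_Turtle is the base turtle actor, leaving the StartMoving event empty for each turtle variety to implement its own movement.
; On BeginPlay it shows a sparks effect at its location and removes it after a short delay.
; It stores a destination point through a setter.
; FinishedMovement marks task completion by playing an explosion effect and sound, then destroys the actor.
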(event `Start Moving`)

(event `self.ReceiveBeginPlay`
  ;[1 1 1] Покажем, что черепашка появилась
  (bind _returnvalue (`GameplayStatics.SpawnEmitterAtLocation` "/Game/StarterContent/Particles/P_Sparks.P_Sparks" (`self.K2_GetActorLocation`)))
  (`KismetSystemLibrary.Delay` 1.0)
  (`ActorComponent.K2_DestroyComponent` _returnvalue))

(fn `Finished Movement`
  (`self.Make Explosion`) ; Покажем, что черепашка справилась со своей задачей
  (`self.K2_DestroyActor`) ; И избавимся от этой черепашки
)

(fn `Make Explosion`
  (bind _returnvalue (`self.K2_GetActorLocation`))
  (`GameplayStatics.SpawnEmitterAtLocation` "/Game/StarterContent/Particles/P_Explosion.P_Explosion" _returnvalue)
  (`GameplayStatics.PlaySoundAtLocation` "/Game/StarterContent/Audio/Explosion_Cue.Explosion_Cue" _returnvalue (struct) 1.0 1.0 0.0 null null null))

(fn `Set Destination Point Location`
  (params (`Destination Point Location` :type "Vector Structure"))
  (set `self.Destination Point Location` `Destination Point Location`))

(fn `UserConstructionScript`)