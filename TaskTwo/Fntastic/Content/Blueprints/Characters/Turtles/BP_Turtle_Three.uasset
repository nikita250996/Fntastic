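; BP_Turtle_Three is a turtle character variant that advances toward its destination in a stop-and-retreat rhythm.
; StartMoving loops AI move requests: one second toward DestinationPointLocation, then half a second back toward StartLocation, which the construction script records.
; Each request is reissued from the immediate exec output after a delay, and reaching the destination calls FinishedMovement without explicitly breaking the loop.
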(event `self.ReceiveBeginPlay`
  (`parent.ReceiveBeginPlay`))

(event `self.Start Moving`
  ;[1 1 1] Эта черепашка секунду идёт вперёд, а потом полсекунды идёт назад
  (`|AIMoveTo` self (`self.Destination Point Location`) null :!label _label
    (:`then`
      (`KismetSystemLibrary.Delay` 1.0)
      (`|AIMoveTo` self (`self.Start Location`) null
        (:`then`
          (`KismetSystemLibrary.Delay` 0.5)
          (goto _label))))
    (:`OnSuccess`
      (`self.Finished Movement`))))

(fn `UserConstructionScript`
  (`parent.UserConstructionScript`)
  (set `self.Start Location` (`self.K2_GetActorLocation`)) ; Начальное положение черепашки
)