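; BP_Turtle_Two is a turtle character Blueprint that travels to a destination point in a stop-and-go rhythm.
; StartMoving issues AIMoveTo toward DestinationPointLocation, lets it run for one second, stops active movement, pauses half a second, then loops back to reissue the move.
; The move's success output calls FinishedMovement.
; BeginPlay and the construction script only call their parent versions.
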(event `self.ReceiveBeginPlay`
  (`parent.ReceiveBeginPlay`))

(event `self.Start Moving`
  ;[1 1 1] Эта черепашка в течение секунды идёт к точке назначения, делает паузу в полсекунды и продолжает движение
  (`|AIMoveTo` self (`self.Destination Point Location`) null :!label _label
    (:`then`
      (`KismetSystemLibrary.Delay` 1.0)
      (`NavMovementComponent.StopActiveMovement` (`self.CharacterMovement`))
      (`KismetSystemLibrary.Delay` 0.5)
      (goto _label))
    (:`OnSuccess`
      (`self.Finished Movement`))))

(fn `UserConstructionScript`
  (`parent.UserConstructionScript`))